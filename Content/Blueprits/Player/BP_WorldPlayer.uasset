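; BP_WorldPlayer is a player Blueprint with a mesh, spring-arm camera boom and follow camera that sets up depth of field at startup.
; On BeginPlay it adds a post-process component at runtime and overrides its aperture, sensor width and focal distance.
; Focal distance copies the boom's arm length once, so it does not track later changes; Tick, overlap and construction logic are empty.
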(event EventBeginPlay
  (bind _returnvalue (AddComponent|AddPostProcessComponent false))
  (Utilities|Struct|SetmembersinPostProcessSettings (Variables|/Script/Engine.PostProcessComponent|GetSettings _returnvalue) 0.5 1.5e+02 (Variables|/Script/Engine.SpringArmComponent|GetTargetArmLength (Variables|Default|GetCameraBoom))))

(event Collision|EventActorBeginOverlap
  (params (OtherActor :type Actor%20Object%20Reference)))

(event EventTick
  (params (DeltaSeconds :type Float%20%28single-precision%29)))

(fn ConstructionScript)