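; BP_Cartel is an interactable sign that shows text from a list in a WB_TextInteract widget, with its mesh set in the construction script.
; TouchingBP hides the player's widget, disables movement input and switches to a mouse-driven, UI-only mode.
; TextToShow displays the current entry, revealing navigation buttons when several exist.
; ExitText removes the widget, recreates the player's widget and restores game input.
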(event Custom|Exit%20text
  (bind _worldplayerref (Variables|Default|GetWorldPlayerRef))
  (bind _playerstate (Variables|/Script/Engine.Pawn|GetPlayerState _worldplayerref))
  (bind _returnvalue (Game|GetPlayerController _playerstate))
  ;[0.15 0.15 0.15 0.5] elimina el widget y reactiva el movimiento al jugador
  (Default|CreateWidget (Variables|Default|GetPlayerRef))
  (Widget|RemovefromParent (Variables|Default|GetWidgetReference))
  (Variables|/Script/Engine.PlayerController|SetbShowMouseCursor (Game|GetPlayerController (Variables|/Script/Engine.Pawn|GetPlayerState (Variables|Default|GetWorldPlayerRef))) false)
  (Input|EnableInput (Variables|Default|GetWorldPlayerRef) _returnvalue)
  (Input|SetInputModeGameOnly _returnvalue false))

(event Custom|Text%20to%20show
  (bind _widgetreference (Variables|Default|GetWidgetReference))
  (bind _listadetextos (Variables|Default|GetListaDeTextos))
  (bind _returnvalue (Utilities|Array|LastIndex _listadetextos))
  ;[0.15 0.15 0.15 0.5] Crea el array de textos y los a;ade
  (if (> _returnvalue 0)
    (Variables|Default|SetTexts_LastIndex _returnvalue)
    (Variables|/Game/UI/Texts/WB_TextInteract.WB_TextInteract_C|SetButtonsVisibility _widgetreference "Visible")
    (else
      (Variables|Default|SetTexts_LastIndex _returnvalue)))
  (Variables|/Game/UI/Texts/WB_TextInteract.WB_TextInteract_C|SetTextToShow _widgetreference (Utilities|Array|Get(acopy) (Variables|Default|GetListaDeTextos) (Variables|Default|GetCurrentText))))

(event EventBeginPlay
  (bind _asbp_world_player (Utilities|Casting|CastToBP_WorldPlayer (Game|GetPlayerCharacter 0)))
  (Variables|Default|SetPlayerRef _asbp_world_player)
  (Class|InteractItem|SavePlayerRef))

(event EventTouchingBP
  (bind _worldplayerref (Variables|Default|GetWorldPlayerRef))
  ;[0.15 0.15 0.15 0.5] crea y a;ade el  widget
  (Default|HiddeWidgetBlueprint (Variables|Default|GetPlayerRef))
  (Input|DisableInput _worldplayerref (Game|GetPlayerController (Variables|/Script/Engine.Pawn|GetPlayerState _worldplayerref))) ; desactiva input
  (bind _returnvalue (UserInterface|CreateWidget "/Game/UI/Texts/WB_TextInteract.WB_TextInteract_C"))
  (Variables|Default|SetWidgetReference _returnvalue)
  (Variables|/Script/Engine.PlayerController|SetbShowMouseCursor (Game|GetPlayerController (Variables|/Script/Engine.Pawn|GetPlayerState (Variables|Default|GetWorldPlayerRef))) true) ; muestra el mouse
  (Input|SetInputModeUIOnly (Game|GetPlayerController (Variables|/Script/Engine.Pawn|GetPlayerState (Variables|Default|GetWorldPlayerRef))) (Variables|Default|GetWidgetReference) "DoNotLock" false) ; setea el input solo para UI
  (UserInterface|Viewport|AddtoViewport (Variables|Default|GetWidgetReference) 0)
  (CallFunction|TexttoShow))

(fn ConstructionScript
  (Components|StaticMesh|SetStaticMesh (Variables|Default|GetStaticMeshComp) (Variables|Default|GetStaticMesh)))