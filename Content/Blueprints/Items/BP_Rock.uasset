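; BP_Rock is a touchable rock item that reacts when touched and feeds the player's rock count to a widget.
; Construction optionally randomizes mesh and scale, sizes the collision box and creates a dynamic material, while BeginPlay sets animation rate from mesh scale.
; Touching plays a material-change montage first and a reaction montage afterwards, plus sound and heart particles at a socket.
; SpawnPlayAnim reuses the material-change branch, and a separate function sets the material parameter.
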(event Custom|SpawnPlayAnim
  (bind _skeletalmeshcomp (Variables|Default|GetSkeletalMeshComp))
  (bind _returnvalue (Transformation|GetSocketTransform _skeletalmeshcomp "ParticleSpamSocket" "RTS_World"))
  (bind (_location _rotation _scale) (Math|Transform|BreakTransform _returnvalue))
  (Animation|Montage|MontagePlay (Components|SkeletalMesh|GetAnimInstance (Variables|Default|GetSkeletalMeshComp)) (Variables|Animations|GetChangeMatMontage) 1.1 "MontageLength" 0.0 true)
  (Variables|Default|SetAlreadyChangeMat true)
  (Class|PlaySoundandParticles|PlaySoundandParticles (Variables|Default|GetObjectEfects) "/Game/Sounds/MS_TouchingOBjects.MS_TouchingOBjects" "/Game/Particles/Interaction_Particles/NS_Hearts.NS_Hearts" self "ParticleSpamSocket" false false _location _rotation (+ _scale "1.000000,1.000000,1.000000")))

(event EventBeginPlay
  (|CallParentFunction)
  (bind _output_get (Variables|Animation|SetConst_MeshSize (Transformation|GetWorldScale (Variables|Default|GetSkeletalMeshComp)))) ; settea la constante de World scale
  (Class|InteractItem|SetAnimRatePlay _output_get 0.9 1.1 1.2 1.3 1.6 1.8 1.0 0.5 0.2) ; Setea la velocidad de animacion dependiendo del tama;o del mesh
)

(event EventTouchingBP
  (bind _worldplayerref (Variables|Default|GetWorldPlayerRef))
  (bind _skeletalmeshcomp (Variables|Default|GetSkeletalMeshComp))
  (bind _returnvalue (Transformation|GetSocketTransform _skeletalmeshcomp "ParticleSpamSocket" "RTS_World"))
  (bind (_location _rotation _scale) (Math|Transform|BreakTransform _returnvalue))
  (|CallParentFunction)
  (bind _outvalue (CallFunction|CheckAlreadyChangeMat (Variables|/Script/MyWorld.WorldPlayer|GetCurrentAmountOfRocks (Variables|Default|GetWorldPlayerRef))) ; despues de esta hay que actualizar el widget en c++ o bp
    (:BO_PinTrue
      _)
    (:BO_PinFalse
      _))
  (bind _output_get (Variables|/Script/MyWorld.WorldPlayer|SetCurrentAmountOfRocks _worldplayerref _outvalue))
  (Class|WorldPlayer|SetAmountOfElementstoWidget _worldplayerref _output_get (Variables|/Script/MyWorld.WorldPlayer|GetCurrentAmountOfFlowers _worldplayerref) (Variables|/Script/MyWorld.WorldPlayer|GetCurrentAmountOfTrees _worldplayerref) (Variables|/Script/MyWorld.WorldPlayer|GetCurrentAmountOfLights _worldplayerref))
  (if (Variables|Default|GetAlreadyChangeMat)
    (Animation|Montage|MontagePlay (Components|SkeletalMesh|GetAnimInstance (Variables|Default|GetSkeletalMeshComp)) (Variables|Animations|GetReactionMontage) 1.0 "MontageLength" 0.0 true)
    (else
      (Animation|Montage|MontagePlay (Components|SkeletalMesh|GetAnimInstance (Variables|Default|GetSkeletalMeshComp)) (Variables|Animations|GetChangeMatMontage) 1.1 "MontageLength" 0.0 true)
      (Variables|Default|SetAlreadyChangeMat true)))
  (Class|PlaySoundandParticles|PlaySoundandParticles (Variables|Default|GetObjectEfects) "/Game/Sounds/MS_TouchingOBjects.MS_TouchingOBjects" "/Game/Particles/Interaction_Particles/NS_Hearts.NS_Hearts" self "ParticleSpamSocket" false false _location _rotation (+ _scale "1.000000,1.000000,1.000000")))

(fn ConstructionScript
  (bind _skeletal_mesh_to_showarray (Variables|Default|GetSkeletal%20Mesh%20To%20ShowArray))
  (|CallParentFunction)
  (if (Variables|Components|SKMesh|GetRandomMesh?)
    (Components|SkeletalMesh|SetSkeletalMeshAsset (Variables|Default|GetSkeletalMeshComp) (Utilities|Array|Get(acopy) _skeletal_mesh_to_showarray (Math|Random|RandomIntegerinRange 0 (Utilities|Array|LastIndex _skeletal_mesh_to_showarray))))
    (Transformation|SetActorScale3D (Math|Conversions|ToVector(Float) (Math|Random|RandomFloatinRange 0.3 1.5)))
    (else
      (Components|SkeletalMesh|SetSkeletalMeshAsset (Variables|Default|GetSkeletalMeshComp) (Variables|Default|GetSkeletalMeshToShow))))
  (Components|Box|SetBoxExtent (Variables|Default|GetBoxComp) (* (Variables|Default|GetCollitionBoxScale) (Variables|Default|GetCollitionBoxScaleMultiplier)) true)
  (bind _returnvalue (Rendering|Material|CreateDynamicMaterialInstance (Variables|Default|GetSkeletalMeshComp) (Variables|Default|GetElementIndex) (Variables|MaterialDynamic|GetMaterial_To_Put_In) "None" :!class /Script/Engine.PrimitiveComponent))
  (Variables|MaterialDynamic|SetMaterialInstanceRef _returnvalue)
  (Rendering|Material|SetScalarParameterValue (Variables|MaterialDynamic|GetMaterialInstanceRef) (Variables|Default|GetMaterialParameterName) 1e+01 :!class /Script/Engine.MaterialInstanceDynamic))

(fn SetMatColorNPlayParticles
  (bind _materialinstanceref (Variables|MaterialDynamic|GetMaterialInstanceRef)
    (:then
      (Rendering|Material|SetScalarParameterValue _materialinstanceref (Variables|Default|GetMaterialParameterName) 0.477379 :!class /Script/Engine.MaterialInstanceDynamic))
    (:else)))

(fn CheckAlreadyChangeMat
  (params (Valuetochange :type Integer))
  (bind _outvalue (|CallParentFunction Valuetochange)
    (:BO_PinTrue
      _)
    (:BO_PinFalse
      _))
  (return (stale _branchresult) _outvalue))