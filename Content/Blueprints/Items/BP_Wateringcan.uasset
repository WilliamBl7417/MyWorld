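; BP_Wateringcan is a watering can item that the player picks up, drops and uses to water plants.
; It starts enlarged with attention visuals active.
; After parent touch logic, a FlipFlop gated on the player's equipable object alternates pickup sound with normal scale, and drop sound.
; Watering calls parent logic, plays the player montage and socket-attached effects, then sets a flag blocking repeats within this Blueprint.
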(event EventBeginPlay
  (Class|InteractItem|SavePlayerRef)
  (Transformation|SetWorldScale3D (Variables|Default|GetSceneComponent) "2.000000,2.000000,2.000000")
  (Class|MovementPlayerAtencionComponent|ActivateVisuals (Variables|Default|GetMovementPlayerAtencionComponent)))

(event EventTouchingBP
  (bind _returnvalue (Transformation|GetActorLocation))
  ;[0.15 0.15 0.15 0.5] Tomar o dropear el objeto, reproducir sonido
  (|CallParentFunction)
  (bind _worldplayerref (Variables|Default|GetWorldPlayerRef)
    (:then
      (Variables|/Script/MyWorld.WorldPlayer|GetEquipableObject _worldplayerref
        (:then
          (Utilities|FlowControl|FlipFlop
            (:A
              (Audio|PlaySoundatLocation "/Game/Sounds/MS_TouchingOBjects.MS_TouchingOBjects" _returnvalue "0, 0, 0" 1.0 1.0 0.0 0 0 0 0)
              (Transformation|SetWorldScale3D (Variables|Default|GetSceneComponent) "1.000000,1.000000,1.000000"))
            (:B
              (Audio|PlaySoundatLocation "/Game/Sounds/MS_Droping.MS_Droping" _returnvalue "0, 0, 0" 1.0 1.0 0.0 0 0 0 0))))
        (:else)))
    (:else)))

(event EventWateringPlantBP
  ;[0.15 0.15 0.15 0.5] Watering Event
  (if (not (Variables|Default|GetbWasWateredRef))
    (|CallParentFunction)
    (Class|WorldPlayer|PlayMontageAnim (Variables|Default|GetWorldPlayerRef) "/Game/Animations/Character/Anim_Watering_Montage.Anim_Watering_Montage")
    (Class|PlaySoundandParticles|PlaySoundandParticles (Variables|Default|GetObjectEfects) 0 "/Game/Particles/Interaction_Particles/NS_FlowerBeingWatering.NS_FlowerBeingWatering" self "HandSocket" false true "0, 0, 0" "0, 0, 0" "0, 0, 0")
    (Variables|Default|SetbWasWateredRef true)))

(fn ConstructionScript)