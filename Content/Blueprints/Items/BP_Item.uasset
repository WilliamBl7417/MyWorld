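; BP_Item is an item Blueprint that refreshes the player's widget counts of rocks, flowers, trees and lights.
; TestFunction passes a value to CheckAlreadyChangeMat, stores the result in ElementIndex, then sends WorldPlayerRef's current totals to SetAmountOfElementsToWidget.
; Both branches of that check are empty.
; TouchingBP and the construction script only call their parent versions, and the default events are disabled.
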(event EventBeginPlay)

(event Collision|EventActorBeginOverlap
  (params (OtherActor :type Actor%20Object%20Reference)))

(event EventTick
  (params (DeltaSeconds :type Float%20%28single-precision%29)))

(event EventTouchingBP
  (|CallParentFunction))

(fn ConstructionScript
  (|CallParentFunction))

(fn TestFunction
  (params (Valuetochange :type Integer))
  (bind _worldplayerref (Variables|Default|GetWorldPlayerRef))
  (bind _outvalue (Class|InteractItem|CheckAlreadyChangeMat Valuetochange) ; despues de esta hay que actualizar el widget en c++ o bp
    (:BO_PinTrue
      _)
    (:BO_PinFalse
      _))
  (Variables|Default|SetElementIndex _outvalue)
  (Class|WorldPlayer|SetAmountOfElementstoWidget _worldplayerref (Variables|/Script/MyWorld.WorldPlayer|GetCurrentAmountOfRocks _worldplayerref) (Variables|/Script/MyWorld.WorldPlayer|GetCurrentAmountOfFlowers _worldplayerref) (Variables|/Script/MyWorld.WorldPlayer|GetCurrentAmountOfTrees _worldplayerref) (Variables|/Script/MyWorld.WorldPlayer|GetCurrentAmountOfLights _worldplayerref)))