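; BP_LIght is a light item, apparently a candle, whose point light flickers at irregular intervals.
; From BeginPlay it prints its owner's name, then loops endlessly through three chained timelines, each preceded by a random delay.
; Each timeline update eases the current intensity slightly toward a fresh random value between configurable minimum and maximum bounds.
; PlaceCandle sets the light to a fixed high intensity, and Tick only stores the delta time.
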(event EventBeginPlay
  (bind _returnvalue (Math|Random|RandomFloatinRange 1.0 2.0))
  (Development|PrintString (Utilities|GetDisplayName (Components|GetOwner)))
  (Utilities|FlowControl|Delay _returnvalue :!label _label)
  (bind _newtrack_0 (Timeline|Timeline PlayFromStart)
    (:Update
      (Rendering|Components|Light|SetIntensity (Variables|Default|GetPointLight) (Math|Float|Lerp (Variables|/Script/Engine.LightComponentBase|GetIntensity (Variables|Default|GetPointLight)) (Math|Random|RandomFloatinRange (Variables|Default|GetIntensity%20ligh%20min) (Variables|Default|GetIntensity%20ligh%20max)) (* _newtrack_0 0.08))))
    (:Finished
      (Utilities|FlowControl|Delay _returnvalue)
      (bind _newtrack_0_2 (Timeline|Timeline_0 PlayFromStart)
        (:Update
          (Rendering|Components|Light|SetIntensity (Variables|Default|GetPointLight) (Math|Float|Lerp (Variables|/Script/Engine.LightComponentBase|GetIntensity (Variables|Default|GetPointLight)) (Math|Random|RandomFloatinRange (Variables|Default|GetIntensity%20ligh%20min) (Variables|Default|GetIntensity%20ligh%20max)) (* _newtrack_0_2 0.08))))
        (:Finished
          (Utilities|FlowControl|Delay _returnvalue)
          (bind _newtrack_0_3 (Timeline|Timeline_1 PlayFromStart)
            (:Update
              (Rendering|Components|Light|SetIntensity (Variables|Default|GetPointLight) (Math|Float|Lerp (Variables|/Script/Engine.LightComponentBase|GetIntensity (Variables|Default|GetPointLight)) (Math|Random|RandomFloatinRange (Variables|Default|GetIntensity%20ligh%20min) (Variables|Default|GetIntensity%20ligh%20max)) (* _newtrack_0_3 0.08))))
            (:Finished
              (goto _label))))))))

(event EventTick
  (params (DeltaSeconds :type Float%20%28single-precision%29))
  (Variables|Default|SetTick DeltaSeconds))

(fn ConstructionScript)

(fn PlaceCandle
  (Rendering|Components|Light|SetIntensity (Variables|Default|GetPointLight) 5e+03))