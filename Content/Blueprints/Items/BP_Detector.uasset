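; BP_Detector is a box trigger that broadcasts the EDChanging event dispatcher when the player character enters it.
; BeginPlay caches the player as BP_WorldPlayer, and each box overlap identifies it by comparing display names rather than object references, printing a debug string for player or non-player.
; The construction script sizes the box from three extent variables.
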(event OnComponentBeginOverlap(Box)
  (params (OverlappedComponent :type Primitive%20Component%20Object%20Reference) (OtherActor :type Actor%20Object%20Reference) (OtherComp :type Primitive%20Component%20Object%20Reference) (OtherBodyIndex :type Integer) (bFromSweep :type Boolean) (SweepResult :type Hit%20Result%20Structure%20%28by%20ref%29))
  (bind _as_bp_world_player (Variables|Default|GetAs%20BP%20World%20Player)
    (:then
      (if (Utilities|Enum|Equal(Enum) (Utilities|GetDisplayName OtherActor) (Utilities|GetDisplayName _as_bp_world_player))
        (Development|PrintString "PLayer")
        (Default|CallEDChanging)
        (else
          (Development|PrintString "Not player"))))
    (:else)))

(event EventBeginPlay
  (bind _asbp_world_player (Utilities|Casting|CastToBP_WorldPlayer (Game|GetPlayerCharacter 0)))
  (Variables|Default|SetAs%20BP%20World%20Player _asbp_world_player))

(event Collision|EventActorBeginOverlap
  (params (OtherActor :type Actor%20Object%20Reference)))

(event EventTick
  (params (DeltaSeconds :type Float%20%28single-precision%29)))

(fn ConstructionScript
  (Components|Box|SetBoxExtent (Variables|Default|GetBox) (Math|Vector|MakeVector (Variables|Boxextend|GetBoxExtendX) (Variables|Boxextend|GetBoxExtendY) (Variables|Boxextend|GetBoxExtendZ)) true))