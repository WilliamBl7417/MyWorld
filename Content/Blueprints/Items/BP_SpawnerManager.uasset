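; BP_SpawnerManager is a manager actor that gathers references to the level's item spawners and the player, but does not yet drive any spawning.
; On BeginPlay it casts the player character to BP_WorldPlayer and, if that succeeds, caches it along with every BP_Spawner found through GetAllActorsOfClass.
; Unconnected nodes for spawner count, current-spawner lookup and the player's WBElementsAmount have no effect.
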(event EventBeginPlay
  (bind _asbp_world_player (Utilities|Casting|CastToBP_WorldPlayer (Game|GetPlayerCharacter 0)))
  (bind _output_get (Variables|Default|SetPlayerReference _asbp_world_player))
  (bind _outactors (Actor|GetAllActorsOfClass "/Game/Blueprints/Items/BP_Spawner.BP_Spawner_C"))
  (Variables|Default|SetBP_Spanwer _outactors))

(fn ConstructionScript)