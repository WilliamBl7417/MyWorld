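; BP_Floor is a floor actor that sets up its mesh and a randomized material in the Construction Script, with no active event logic.
; It assigns the chosen mesh to RealMesh and ShadowMesh, but applies the scale multiplier and dynamic material only to RealMesh.
; Random PDO, tiling and texture-blend power parameters vary the look, re-rolling whenever construction runs.
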(event EventBeginPlay)

(event Collision|EventActorBeginOverlap
  (params (OtherActor :type Actor%20Object%20Reference)))

(event EventTick
  (params (DeltaSeconds :type Float%20%28single-precision%29)))

(fn ConstructionScript
  (bind _meshtoshow (Variables|MeshVariables|GetMeshToShow))
  (Components|StaticMesh|SetStaticMesh (Variables|Default|GetReal_Mesh) _meshtoshow)
  (Components|StaticMesh|SetStaticMesh (Variables|Default|GetShadow_Mesh) _meshtoshow)
  (Transformation|SetWorldScale3D (Variables|Default|GetReal_Mesh) (* (Variables|MeshVariables|GetScale_static_mesh) (Variables|MeshVariables|GetStaticMeshScaleMultiplyer)))
  (bind _returnvalue (Rendering|Material|CreateDynamicMaterialInstance (Variables|Default|GetReal_Mesh) (Variables|MaterialVariables|GetElementIndex) (Variables|MaterialVariables|GetMaterial) "None" :!class /Script/Engine.PrimitiveComponent))
  (Variables|MaterialVariables|SetMaterial%20instance%20reference _returnvalue)
  (Utilities|FlowControl|Sequence
    (:then_0
      (Rendering|Material|SetScalarParameterValue (Variables|MaterialVariables|GetMaterial%20instance%20reference) (Variables|MaterialVariables|GetParameterNameForPDO) (Math|Random|RandomFloatinRange 1e+01 16.0) :!class /Script/Engine.MaterialInstanceDynamic))
    (:then_1
      (Rendering|Material|SetScalarParameterValue (Variables|MaterialVariables|GetMaterial%20instance%20reference) (Variables|MaterialVariables|GetTillingTwoColors) (Math|Random|RandomFloatinRange 0.1 2.0) :!class /Script/Engine.MaterialInstanceDynamic)
      (Rendering|Material|SetScalarParameterValue (Variables|MaterialVariables|GetMaterial%20instance%20reference) (Variables|Default|GetPower_two%20textures) (Math|Random|RandomFloatinRange 5.0 7.0) :!class /Script/Engine.MaterialInstanceDynamic))))