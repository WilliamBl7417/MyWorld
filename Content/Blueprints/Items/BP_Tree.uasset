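; Interactive tree item that plays heart particles and sound on each touch and can switch from a dark base color to its own colors.
; The construction script sets the configurable skeletal mesh and creates a dynamic MI_Trees material with the dark starting look.
; TouchingBP plays the material-change montage only on first touch, guarded by a flag.
; A separate ChangeMaterialInteraction event applies the main and edge-wear colors.
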(event EventTouchingBP
  (if (Variables|Default|GetAlreadyChangeMat)
    (Class|PlaySoundandParticles|PlaySoundandParticles (Variables|Default|GetObjectEfects) 0 "/Game/Particles/Interaction_Particles/NS_Hearts.NS_Hearts" self "ParticlesSocket" true false "0, 0, 0" "0, 0, 0" "0, 0, 0")
    (else
      (Class|PlaySoundandParticles|PlaySoundandParticles (Variables|Default|GetObjectEfects) 0 "/Game/Particles/Interaction_Particles/NS_Hearts.NS_Hearts" self "ParticlesSocket" true false "0, 0, 0" "0, 0, 0" "0, 0, 0")
      (Animation|Montage|MontagePlay (Components|SkeletalMesh|GetAnimInstance (Variables|Default|GetSkeletalMeshComp)) "/Game/Animations/Tree/Anim_ChangingMaterial_Montage.Anim_ChangingMaterial_Montage" 1.0 "MontageLength" 0.0 true)
      (Variables|Default|SetAlreadyChangeMat true))))

(event EventChangeMaterialInteraction
  ;[0.15 0.15 0.15 0.5] Set Material change
  (Rendering|Material|SetVectorParameterValue (Variables|Default|GetMaterialInstanceRef) "Color_EdgeWear" (Variables|Default|GetEdgeColor) :!class /Script/Engine.MaterialInstanceDynamic)
  (Rendering|Material|SetVectorParameterValue (Variables|Default|GetMaterialInstanceRef) "Main_Color" (Variables|Default|GetMainColor) :!class /Script/Engine.MaterialInstanceDynamic))

(fn ConstructionScript
  (bind _skeletalmeshcomp (Variables|Default|GetSkeletalMeshComp))
  (Components|SkeletalMesh|SetSkeletalMeshAsset _skeletalmeshcomp (Variables|Default|GetSkeletalMeshToShow))
  (bind _returnvalue (Rendering|Material|CreateDynamicMaterialInstance _skeletalmeshcomp 0 "/Game/Materials/MI_Trees.MI_Trees" "None" :!class /Script/Engine.PrimitiveComponent))
  (bind _output_get (Variables|Default|SetMaterialInstanceRef _returnvalue))
  (Rendering|Material|SetVectorParameterValue _output_get "Color_EdgeWear" (Variables|Default|GetEdgeColor) :!class /Script/Engine.MaterialInstanceDynamic)
  (Rendering|Material|SetVectorParameterValue _output_get "Main_Color" "(R=0.161458,G=0.142768,B=0.135390,A=1.000000)" :!class /Script/Engine.MaterialInstanceDynamic)
  (Rendering|Material|SetScalarParameterValue _output_get "Edgeweare_Adjustment" -0.48 :!class /Script/Engine.MaterialInstanceDynamic))