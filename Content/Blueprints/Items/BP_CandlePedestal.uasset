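; Pedestal item that accepts a candle and reacts to touch with heart effects, or broken hearts while it is empty.
; Placing swaps the candle for a stripped copy snapped to the attach point and notifies that copy's light reference.
; A successful placement, or a touch once filled, spawns BP_LIght actors at random points around LightsUp up to a small cap, then destroys them one by one on a delay.
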(event EventBeginPlay)

(event EventTouchingBP
  (bind _staticmeshcomp (Variables|Default|GetStaticMeshComp))
  (bind _staticmeshcomp_2 (Variables|Default|GetStaticMeshComp))
  (bind _limitslightspawn (Variables|Default|GetLimitsLightSpawn))
  (bind _array (Variables|Default|Getarray))
  (bind _lights_up (Variables|Default|GetLights%20up))
  (bind _returnvalue (Transformation|GetWorldTransform _staticmeshcomp))
  (bind _returnvalue_2 (Transformation|GetWorldTransform _lights_up))
  (bind _returnvalue_3 (Transformation|GetWorldTransform _staticmeshcomp_2))
  (bind (_x _y _z) (Math|Vector|BreakVector (.location _returnvalue_2)))
  (|CallParentFunction)
  (if (Variables|Default|GetbIsCandlePlaced)
    (Class|PlaySoundandParticles|PlaySoundandParticles (Variables|Default|GetObjectEfects) "/Game/Sounds/MS_Error.MS_Error" "/Game/Particles/Interaction_Particles/NS_Hearts.NS_Hearts" 0 "None" false false (.location _returnvalue) (.rotation _returnvalue) (.scale _returnvalue))
    ;[0.15 0.15 0.15 0.5] Spawnea luz alrededor del pedestal
    (if (> (Variables|Default|GetCandleAmount) 3) :!label _label
      ;[0.15 0.15 0.15 0.5] elimina las candelas alrededor del pedestal
      (Utilities|FlowControl|Delay 3.0 :!label _label_2)
      (Variables|Default|SetNewVar (Utilities|Array|Get(acopy) _array (Utilities|Array|LastIndex _array)))
      (Utilities|Array|RemoveItem _array (Variables|Default|GetNewVar))
      (Utilities|IsValid (Variables|Default|GetNewVar)
        (:Is%20Valid
          (Actor|DestroyActor (Variables|Default|GetNewVar))
          (Variables|Default|SetCandleAmount (- (Variables|Default|GetCandleAmount) 1))
          (if (not (== (Utilities|Array|Length (Variables|Default|Getarray)) 0))
            (goto _label_2))))
      (else
        (bind _returnvalue_4 (Game|SpawnActorfromClass "/Game/Blueprints/Items/BP_LIght.BP_LIght_C" (Math|Transform|MakeTransform (Math|Vector|MakeVector (Math|Random|RandomFloatinRange (- _x _limitslightspawn) (+ _x _limitslightspawn)) (Math|Random|RandomFloatinRange (- _y _limitslightspawn) (+ _y _limitslightspawn)) (Math|Random|RandomFloatinRange (- _z _limitslightspawn) (+ _z _limitslightspawn))) (.rotation _returnvalue_2) (.scale _returnvalue_2)) "Undefined" "MultiplyWithRoot" 0 0))
        (Utilities|Array|Add (Variables|Default|Getarray) _returnvalue_4)
        (Variables|Default|SetCandleAmount (+ (Variables|Default|GetCandleAmount) 1))
        (goto _label)))
    (else
      (Class|PlaySoundandParticles|PlaySoundandParticles (Variables|Default|GetObjectEfects) "/Game/Sounds/MS_Error.MS_Error" "/Game/Particles/Interaction_Particles/NS_BrockenHearts.NS_BrockenHearts" 0 "None" false false (.location _returnvalue_3) (.rotation _returnvalue_3) (.scale _returnvalue_3)))))

(event EventPlaceCandleBP
  (params (CandleToPlace :type Candle%20Object%20Reference))
  (bind _staticmeshcomp (Variables|Default|GetStaticMeshComp))
  (bind _limitslightspawn (Variables|Default|GetLimitsLightSpawn))
  (bind _array (Variables|Default|Getarray))
  (bind _lights_up (Variables|Default|GetLights%20up))
  (bind _returnvalue (Transformation|GetWorldTransform _staticmeshcomp))
  (bind _returnvalue_2 (Transformation|GetWorldTransform _lights_up))
  (bind (_x _y _z) (Math|Vector|BreakVector (.location _returnvalue_2)))
  ;[0.15 0.15 0.15 0.5] logica para poner la candela en sul ugar
  (if (not (Variables|Default|GetbIsCandlePlaced))
    (Class|Candle|DestroyCandle CandleToPlace)
    (bind _returnvalue_3 (Game|SpawnActorfromClass "/Game/Blueprints/Items/BP_Candle.BP_Candle_C" (Transformation|GetWorldTransform (Variables|Default|GetCandleAttachPoint)) "Undefined" "MultiplyWithRoot" 0 0))
    (Class|MovementPlayerAtencionComponent|DeactivateVisuals (Variables|/Script/MyWorld.Candle|GetMovementPlayerAtentionComponent _returnvalue_3))
    (Transformation|AttachComponentToComponent _returnvalue_3 (Variables|Default|GetCandleAttachPoint) "None" "SnapToTarget" "SnapToTarget" "SnapToTarget" true)
    (Variables|Default|SetbIsCandlePlaced true)
    (Utilities|FlowControl|Delay 0.1)
    (Default|DestroyComponents _returnvalue_3)
    (bind _ligtreference (Variables|/Game/Blueprints/Items/BP_Candle.BP_Candle_C|GetLigtReference _returnvalue_3)
      (:then
        (Default|PlaceCandle _ligtreference)
        (Class|PlaySoundandParticles|PlaySoundandParticles (Variables|Default|GetObjectEfects) "/Game/Sounds/MS_Error.MS_Error" "/Game/Particles/Interaction_Particles/NS_Hearts.NS_Hearts" 0 "None" false false (.location _returnvalue) (.rotation _returnvalue) (.scale _returnvalue))
        ;[0.15 0.15 0.15 0.5] Spawnea luz alrededor del pedestal
        (if (> (Variables|Default|GetCandleAmount) 3) :!label _label
          ;[0.15 0.15 0.15 0.5] elimina las candelas alrededor del pedestal
          (Utilities|FlowControl|Delay 3.0 :!label _label_2)
          (Variables|Default|SetNewVar (Utilities|Array|Get(acopy) _array (Utilities|Array|LastIndex _array)))
          (Utilities|Array|RemoveItem _array (Variables|Default|GetNewVar))
          (Utilities|IsValid (Variables|Default|GetNewVar)
            (:Is%20Valid
              (Actor|DestroyActor (Variables|Default|GetNewVar))
              (Variables|Default|SetCandleAmount (- (Variables|Default|GetCandleAmount) 1))
              (if (not (== (Utilities|Array|Length (Variables|Default|Getarray)) 0))
                (goto _label_2))))
          (else
            (bind _returnvalue_4 (Game|SpawnActorfromClass "/Game/Blueprints/Items/BP_LIght.BP_LIght_C" (Math|Transform|MakeTransform (Math|Vector|MakeVector (Math|Random|RandomFloatinRange (- _x _limitslightspawn) (+ _x _limitslightspawn)) (Math|Random|RandomFloatinRange (- _y _limitslightspawn) (+ _y _limitslightspawn)) (Math|Random|RandomFloatinRange (- _z _limitslightspawn) (+ _z _limitslightspawn))) (.rotation _returnvalue_2) (.scale _returnvalue_2)) "Undefined" "MultiplyWithRoot" 0 0))
            (Utilities|Array|Add (Variables|Default|Getarray) _returnvalue_4)
            (Variables|Default|SetCandleAmount (+ (Variables|Default|GetCandleAmount) 1))
            (goto _label))))
      (:else))))

(fn ConstructionScript
  (Components|StaticMesh|SetStaticMesh (Variables|Default|GetStaticMeshComp) (Variables|Default|GetStaticMesh)))