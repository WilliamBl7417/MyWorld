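; Interactive flower that starts with grayscale materials and reacts to the player watering or touching it.
; Watering updates the player's flower count and widget, then plays either a material-change montage with camera shake or the touch reaction, depending on WasWatered.
; Touching shows hearts if watered, otherwise broken hearts, or swaps to colored materials in level four.
; ChangeMaterialInteraction also triggers the color swap, and BeginPlay requests a scale-based animation rate.
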(event Custom|SetAnimSpeed
  ;[0.15 0.15 0.15 0.5] Settea la velocidad de animacion dependiendo del tam;o del SK mesh
  (Class|InteractItem|SetAnimRatePlay (Variables|Default|GetInitialScale) 0.8 1.0 0.7 1.0 0.9 1.0 1.5 1.0 0.9))

(event Custom|TriggerInteraction
  (bind _skeletalmeshcomp (Variables|Default|GetSkeletalMeshComp))
  ;[0.15 0.15 0.15 0.5] Si no sido regada, Riega y  reproduce animacion y sonidos y efectos
  (if (Variables|Default|GetbWasWatered)
    (if (Variables|Default|GetbWasWatered)
      ;[0.15 0.15 0.15 0.5] reproduce sonido y particulas despues de ser regada
      (|CallParentFunction)
      (Animation|Montage|PlayMontage (Variables|Default|GetSkeletalMeshComp) "/Game/Animations/Flower/Anim_Flower_Reacting_Montage.Anim_Flower_Reacting_Montage"
        (:then
          (Class|PlaySoundandParticles|PlaySoundandParticles (Variables|Default|GetObjectEfects) 0 "/Game/Particles/Interaction_Particles/NS_Hearts.NS_Hearts" self "ParticlesSocket" true false "0, 0, 0" "0, 0, 0" "0, 0, 0")))
      (else
        (|CallParentFunction)
        (if (Variables|Default|GetIsLvLFour?)
          ;[0.15 0.15 0.15 0.5] Cambia el material de gris a los colores
          (Rendering|Material|SetMaterial _skeletalmeshcomp 0 "/Game/Materials/Foliage_Materials/Flowe_M/MI_Flowers_Flower_C.MI_Flowers_Flower_C")
          (Rendering|Material|SetMaterial _skeletalmeshcomp 1 "/Game/Materials/Foliage_Materials/Flowe_M/MI_Flowers_Center_C.MI_Flowers_Center_C")
          (Rendering|Material|SetMaterial _skeletalmeshcomp 2 "/Game/Materials/Foliage_Materials/Flowe_M/MI_Flowers_Tallo_C.MI_Flowers_Tallo_C")
          (Rendering|Material|SetMaterial _skeletalmeshcomp 3 "/Game/Materials/Foliage_Materials/Flowe_M/MI_Grass_Flower.MI_Grass_Flower")
          (Variables|Default|SetAlreadyChangeMat true)
          (Class|PlaySoundandParticles|PlayOnlyParticles (Variables|Default|GetObjectEfects) "/Game/Particles/SmokeEffects/VFX_Flowers.VFX_Flowers" 0 "ParticlesSocket" (Transformation|GetActorLocation) "0, 0, 0" false)
          (else
            ;[0.15 0.15 0.15 0.5] Reproduce lsonido y particulas en la locacion asignada antes de ser regada
            (Animation|Montage|PlayMontage (Variables|Default|GetSkeletalMeshComp) "/Game/Animations/Flower/Anim_Flower_Reacting_Montage.Anim_Flower_Reacting_Montage"
              (:then
                (Class|PlaySoundandParticles|PlaySoundandParticles (Variables|Default|GetObjectEfects) 0 "/Game/Particles/Interaction_Particles/NS_BrockenHearts.NS_BrockenHearts" self "ParticlesSocket" true false "0, 0, 0" "0, 0, 0" "0, 0, 0")))))))
    (else
      (Animation|Montage|MontagePlay (Components|SkeletalMesh|GetAnimInstance (Variables|Default|GetSkeletalMeshComp)) "/Game/Animations/Flower/Anim_Flower_ChangingMat_Montage.Anim_Flower_ChangingMat_Montage" 1.1 "MontageLength" 0.0 true)
      (Class|PlaySoundandParticles|PlaySoundandParticles (Variables|Default|GetObjectEfects) 0 "/Game/Particles/Interaction_Particles/NS_Hearts.NS_Hearts" self "ParticlesSocket" true false "0, 0, 0" "0, 0, 0" "0, 0, 0")
      (Game|Feedback|ClientStartCameraShake (Game|GetPlayerController 0) "/Game/Animations/Character/CS_FeedBack.CS_FeedBack_C" 1e+01 "World" "0, 0, 0"))))

(event EventBeginPlay
  ;[0.15 0.15 0.15 0.5] Crea las referencias del jugador
  (bind _asbp_world_player (Utilities|Casting|CastToBP_WorldPlayer (Game|GetPlayerCharacter 0)))
  (Variables|Default|SetAs%20BP%20World%20Player _asbp_world_player)
  (Class|InteractItem|SavePlayerRef _asbp_world_player)
  ;[0.15 0.15 0.15 0.5] Settea parametros iniciales
  (CallFunction|SetAnimSpeed)
  (Variables|Default|SetInitialScale (Transformation|GetWorldScale (Variables|Default|GetSkeletalMeshComp)))
  (bind _returnvalue (Game|GetCurrentLevelName true))
  (if (Utilities|Enum|Equal(Enum) _returnvalue "LvL_Four")
    (Variables|Default|SetShoulPlaySound false)))

(event EventChangeMaterialInteraction
  (bind _skeletalmeshcomp (Variables|Default|GetSkeletalMeshComp))
  ;[0.15 0.15 0.15 0.5] Cambia el material de gris a los colores
  (Rendering|Material|SetMaterial _skeletalmeshcomp 0 "/Game/Materials/Foliage_Materials/Flowe_M/MI_Flowers_Flower_C.MI_Flowers_Flower_C")
  (Rendering|Material|SetMaterial _skeletalmeshcomp 1 "/Game/Materials/Foliage_Materials/Flowe_M/MI_Flowers_Center_C.MI_Flowers_Center_C")
  (Rendering|Material|SetMaterial _skeletalmeshcomp 2 "/Game/Materials/Foliage_Materials/Flowe_M/MI_Flowers_Tallo_C.MI_Flowers_Tallo_C")
  (Rendering|Material|SetMaterial _skeletalmeshcomp 3 "/Game/Materials/Foliage_Materials/Flowe_M/MI_Grass_Flower.MI_Grass_Flower")
  (Variables|Default|SetAlreadyChangeMat true)
  (Class|PlaySoundandParticles|PlayOnlyParticles (Variables|Default|GetObjectEfects) "/Game/Particles/SmokeEffects/VFX_Flowers.VFX_Flowers" 0 "ParticlesSocket" (Transformation|GetActorLocation) "0, 0, 0" false))

(event EventTouchingBP
  (bind _skeletalmeshcomp (Variables|Default|GetSkeletalMeshComp))
  (if (Variables|Default|GetbWasWatered)
    ;[0.15 0.15 0.15 0.5] reproduce sonido y particulas despues de ser regada
    (|CallParentFunction)
    (Animation|Montage|PlayMontage (Variables|Default|GetSkeletalMeshComp) "/Game/Animations/Flower/Anim_Flower_Reacting_Montage.Anim_Flower_Reacting_Montage"
      (:then
        (Class|PlaySoundandParticles|PlaySoundandParticles (Variables|Default|GetObjectEfects) 0 "/Game/Particles/Interaction_Particles/NS_Hearts.NS_Hearts" self "ParticlesSocket" true false "0, 0, 0" "0, 0, 0" "0, 0, 0")))
    (else
      (|CallParentFunction)
      (if (Variables|Default|GetIsLvLFour?)
        ;[0.15 0.15 0.15 0.5] Cambia el material de gris a los colores
        (Rendering|Material|SetMaterial _skeletalmeshcomp 0 "/Game/Materials/Foliage_Materials/Flowe_M/MI_Flowers_Flower_C.MI_Flowers_Flower_C")
        (Rendering|Material|SetMaterial _skeletalmeshcomp 1 "/Game/Materials/Foliage_Materials/Flowe_M/MI_Flowers_Center_C.MI_Flowers_Center_C")
        (Rendering|Material|SetMaterial _skeletalmeshcomp 2 "/Game/Materials/Foliage_Materials/Flowe_M/MI_Flowers_Tallo_C.MI_Flowers_Tallo_C")
        (Rendering|Material|SetMaterial _skeletalmeshcomp 3 "/Game/Materials/Foliage_Materials/Flowe_M/MI_Grass_Flower.MI_Grass_Flower")
        (Variables|Default|SetAlreadyChangeMat true)
        (Class|PlaySoundandParticles|PlayOnlyParticles (Variables|Default|GetObjectEfects) "/Game/Particles/SmokeEffects/VFX_Flowers.VFX_Flowers" 0 "ParticlesSocket" (Transformation|GetActorLocation) "0, 0, 0" false)
        (else
          ;[0.15 0.15 0.15 0.5] Reproduce lsonido y particulas en la locacion asignada antes de ser regada
          (Animation|Montage|PlayMontage (Variables|Default|GetSkeletalMeshComp) "/Game/Animations/Flower/Anim_Flower_Reacting_Montage.Anim_Flower_Reacting_Montage"
            (:then
              (Class|PlaySoundandParticles|PlaySoundandParticles (Variables|Default|GetObjectEfects) 0 "/Game/Particles/Interaction_Particles/NS_BrockenHearts.NS_BrockenHearts" self "ParticlesSocket" true false "0, 0, 0" "0, 0, 0" "0, 0, 0"))))))))

(event EventWateringPlantBP
  (bind _worldplayerref (Variables|Default|GetWorldPlayerRef))
  (bind _skeletalmeshcomp (Variables|Default|GetSkeletalMeshComp))
  (|CallParentFunction)
  (Utilities|FlowControl|Sequence
    (:then_0
      (bind _outvalue (Class|InteractItem|CheckAlreadyChangeMat (Variables|/Script/MyWorld.WorldPlayer|GetCurrentAmountOfFlowers (Variables|Default|GetWorldPlayerRef))) ; despues de esta hay que actualizar el widget en c++ o bp
        (:BO_PinTrue
          _)
        (:BO_PinFalse
          _))
      ;[0.15 0.15 0.15 0.5] Settea parametros en widget y spawner controller
      (Variables|/Script/MyWorld.WorldPlayer|SetCurrentAmountOfFlowers _worldplayerref _outvalue)
      (Class|WorldPlayer|SetAmountOfElementstoWidget _worldplayerref (Variables|/Script/MyWorld.WorldPlayer|GetCurrentAmountOfRocks _worldplayerref) (Variables|/Script/MyWorld.WorldPlayer|GetCurrentAmountOfFlowers _worldplayerref) (Variables|/Script/MyWorld.WorldPlayer|GetCurrentAmountOfTrees _worldplayerref) (Variables|/Script/MyWorld.WorldPlayer|GetCurrentAmountOfLights _worldplayerref))
      ;[0.15 0.15 0.15 0.5] Si no sido regada, Riega y  reproduce animacion y sonidos y efectos
      (if (Variables|Default|GetbWasWatered)
        (if (Variables|Default|GetbWasWatered)
          ;[0.15 0.15 0.15 0.5] reproduce sonido y particulas despues de ser regada
          (|CallParentFunction)
          (Animation|Montage|PlayMontage (Variables|Default|GetSkeletalMeshComp) "/Game/Animations/Flower/Anim_Flower_Reacting_Montage.Anim_Flower_Reacting_Montage"
            (:then
              (Class|PlaySoundandParticles|PlaySoundandParticles (Variables|Default|GetObjectEfects) 0 "/Game/Particles/Interaction_Particles/NS_Hearts.NS_Hearts" self "ParticlesSocket" true false "0, 0, 0" "0, 0, 0" "0, 0, 0")))
          (else
            (|CallParentFunction)
            (if (Variables|Default|GetIsLvLFour?)
              ;[0.15 0.15 0.15 0.5] Cambia el material de gris a los colores
              (Rendering|Material|SetMaterial _skeletalmeshcomp 0 "/Game/Materials/Foliage_Materials/Flowe_M/MI_Flowers_Flower_C.MI_Flowers_Flower_C")
              (Rendering|Material|SetMaterial _skeletalmeshcomp 1 "/Game/Materials/Foliage_Materials/Flowe_M/MI_Flowers_Center_C.MI_Flowers_Center_C")
              (Rendering|Material|SetMaterial _skeletalmeshcomp 2 "/Game/Materials/Foliage_Materials/Flowe_M/MI_Flowers_Tallo_C.MI_Flowers_Tallo_C")
              (Rendering|Material|SetMaterial _skeletalmeshcomp 3 "/Game/Materials/Foliage_Materials/Flowe_M/MI_Grass_Flower.MI_Grass_Flower")
              (Variables|Default|SetAlreadyChangeMat true)
              (Class|PlaySoundandParticles|PlayOnlyParticles (Variables|Default|GetObjectEfects) "/Game/Particles/SmokeEffects/VFX_Flowers.VFX_Flowers" 0 "ParticlesSocket" (Transformation|GetActorLocation) "0, 0, 0" false)
              (else
                ;[0.15 0.15 0.15 0.5] Reproduce lsonido y particulas en la locacion asignada antes de ser regada
                (Animation|Montage|PlayMontage (Variables|Default|GetSkeletalMeshComp) "/Game/Animations/Flower/Anim_Flower_Reacting_Montage.Anim_Flower_Reacting_Montage"
                  (:then
                    (Class|PlaySoundandParticles|PlaySoundandParticles (Variables|Default|GetObjectEfects) 0 "/Game/Particles/Interaction_Particles/NS_BrockenHearts.NS_BrockenHearts" self "ParticlesSocket" true false "0, 0, 0" "0, 0, 0" "0, 0, 0")))))))
        (else
          (Animation|Montage|MontagePlay (Components|SkeletalMesh|GetAnimInstance (Variables|Default|GetSkeletalMeshComp)) "/Game/Animations/Flower/Anim_Flower_ChangingMat_Montage.Anim_Flower_ChangingMat_Montage" 1.1 "MontageLength" 0.0 true)
          (Class|PlaySoundandParticles|PlaySoundandParticles (Variables|Default|GetObjectEfects) 0 "/Game/Particles/Interaction_Particles/NS_Hearts.NS_Hearts" self "ParticlesSocket" true false "0, 0, 0" "0, 0, 0" "0, 0, 0")
          (Game|Feedback|ClientStartCameraShake (Game|GetPlayerController 0) "/Game/Animations/Character/CS_FeedBack.CS_FeedBack_C" 1e+01 "World" "0, 0, 0"))))))

(fn ConstructionScript
  (bind _skeletalmeshcomp (Variables|Default|GetSkeletalMeshComp))
  (Components|StaticMesh|SetStaticMesh (Variables|Default|GetStaticMeshComp) (Variables|Default|GetStaticMesh))
  (Components|SkeletalMesh|SetSkeletalMeshAsset (Variables|Default|GetSkeletalMeshComp) (Variables|Default|GetSkeletalMeshToShow))
  ;[0.15 0.15 0.15 0.5] Settear Materiales escala de grises
  (Rendering|Material|SetMaterial _skeletalmeshcomp 0 "/Game/Materials/Foliage_Materials/Flowe_M/MI_Flowers_Flower_G.MI_Flowers_Flower_G") ; Fower
  (Rendering|Material|SetMaterial _skeletalmeshcomp 1 "/Game/Materials/Foliage_Materials/Flowe_M/MI_Flowers_Center_G.MI_Flowers_Center_G") ; Center Flower
  (Rendering|Material|SetMaterial _skeletalmeshcomp 2 "/Game/Materials/Foliage_Materials/Flowe_M/MI_Flowers_Tallo_G.MI_Flowers_Tallo_G") ; Tallo
  (Rendering|Material|SetMaterial _skeletalmeshcomp 3 "/Game/Materials/Foliage_Materials/Flowe_M/MI_Grass_Flower_G.MI_Grass_Flower_G") ; FlowerGrass
)