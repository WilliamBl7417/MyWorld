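; Player character Blueprint that interacts with world trees, rocks, flowers and lights, tracking their amounts in a HUD widget and calling a respawn when trees drop to half.
; A per-tick camera-to-hair trace fades occluding trees through material parameters.
; BeginPlay adds tilt-shift depth of field and parks two prop-activating box colliders out of reach outside LvL_Four.
; It also opens the pause menu and plays interaction montages, turning toward the target.
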(event OnComponentBeginOverlap(Box)
  (params (OverlappedComponent :type Primitive%20Component%20Object%20Reference) (OtherActor :type Actor%20Object%20Reference) (OtherComp :type Primitive%20Component%20Object%20Reference) (OtherBodyIndex :type Integer) (bFromSweep :type Boolean) (SweepResult :type Hit%20Result%20Structure%20%28by%20ref%29))
  ;[0.15 0.15 0.15 0.5] Collision de los box detecto del ultimo nivel
  (CallFunction|FActivatePropsLastLevel OtherActor))

(event OnComponentBeginOverlap(Box1)
  (params (OverlappedComponent :type Primitive%20Component%20Object%20Reference) (OtherActor :type Actor%20Object%20Reference) (OtherComp :type Primitive%20Component%20Object%20Reference) (OtherBodyIndex :type Integer) (bFromSweep :type Boolean) (SweepResult :type Hit%20Result%20Structure%20%28by%20ref%29))
  ;[0.15 0.15 0.15 0.5] Collision de los box detecto del ultimo nivel
  (CallFunction|FActivatePropsLastLevel OtherActor))

(event Custom|SetInitialRelativeLocation%28LastLevelColliders%29
  ;[0.15 0.15 0.15 0.5] setea la posicion  de los box collider del level 4
  (bind _returnvalue (Game|GetCurrentLevelName true))
  (if (Utilities|Enum|Equal(Enum) _returnvalue "LvL_Four")
    (Transformation|SetRelativeLocation (Variables|Default|GetBox1) (Variables|Default|GetInitial%20Relative%20Location) false false)
    (Transformation|SetRelativeLocation (Variables|Default|GetBox) (Variables|Default|GetInitial%20Relative%20Location2) false false)
    (else
      (Transformation|SetRelativeLocation (Variables|Default|GetBox1) (+ (Variables|/Script/Engine.SceneComponent|GetRelativeLocation (Variables|Default|GetBox1)) "0.000000,0.000000,111600.000000") false false)
      (Transformation|SetRelativeLocation (Variables|Default|GetBox) (+ (Variables|/Script/Engine.SceneComponent|GetRelativeLocation (Variables|Default|GetBox)) "0.000000,0.000000,111600.000000") false false))))

(event Custom|SaveInitialRelativeLocation
  ;[0.15 0.15 0.15 0.5] setea la posicion  de los box collider del level 4
  (Variables|Default|SetInitial%20Relative%20Location (Variables|/Script/Engine.SceneComponent|GetRelativeLocation (Variables|Default|GetBox1)))
  (Variables|Default|SetInitial%20Relative%20Location2 (Variables|/Script/Engine.SceneComponent|GetRelativeLocation (Variables|Default|GetBox))))

(event Custom|Create%20widget
  ;[0.15 0.15 0.15 0.5] Widgets Logic
  (Variables|Widgets|GetWB_ElementsAmount
    (:then
      _)
    (:else
      (bind _returnvalue (UserInterface|CreateWidget "/Game/UI/Texts/WB_ElementsManager.WB_ElementsManager_C"))
      (bind _output_get (Variables|Widgets|SetWB_ElementsAmount _returnvalue))))
  (UserInterface|Viewport|AddtoViewport _output_get 0))

(event Custom|HiddeWidgetBlueprint
  ;[0.15 0.15 0.15 0.5] Widgets Logic
  (Widget|RemovefromParent (Variables|Widgets|GetWB_ElementsAmount)))

(event Custom|ReLoadPreviusWidget
  (bind _returnvalue (Game|GetPlayerController 0))
  (Widget|RemovefromParent (Variables|Widgets|GetPause))
  (Variables|/Script/Engine.PlayerController|SetbShowMouseCursor _returnvalue false)
  (UserInterface|Viewport|AddtoViewport (Variables|Widgets|GetWB_ElementsAmount) 0)
  (Input|EnableInput _returnvalue))

(event Input|EnhancedActionEvents|EnhancedInputActionIA_Jump
  (params (ActionValue :type Boolean) (ElapsedSeconds :type Float%20%28double-precision%29) (TriggeredSeconds :type Float%20%28double-precision%29) (InputAction :type Input%20Action%20Object%20Reference :default "/Game/Blueprints/Player/Inputs/IA_Jump.IA_Jump"))
  (bind _returnvalue (Game|GetPlayerController 0))
  (:Started
    (bind _returnvalue_2 (UserInterface|CreateWidget "/Game/Blueprints/GameMode/Menu/WB_PauseMenu.WB_PauseMenu_C" (Game|GetPlayerController 0)))
    (bind _output_get (Variables|Widgets|SetPause _returnvalue_2))
    (Variables|/Script/Engine.PlayerController|SetbShowMouseCursor _returnvalue true)
    (UserInterface|Viewport|AddtoViewport _output_get 0)
    (Input|DisableInput _returnvalue)))

(event EventBeginPlay
  ;[0.15 0.15 0.15 0.5] Setea la camara Style
  (bind _returnvalue (AddComponent|AddPostProcessComponent false))
  (Utilities|Struct|SetmembersinPostProcessSettings (Variables|/Script/Engine.PostProcessComponent|GetSettings _returnvalue) 3.0 8e+02 (Variables|/Script/Engine.SpringArmComponent|GetTargetArmLength (Variables|Default|GetCameraBoom))) ; setea la camara til-shilf
  (Utilities|FlowControl|Sequence
    (:then_0
      (CallFunction|SaveInitialRelativeLocation))
    (:then_1
      (CallFunction|SetInitialRelativeLocation(LastLevelColliders)))
    (:then_2
      (CallFunction|CreateWidget))))

(event EventPlayMontageAnim
  (params (MontageToPlay :type Anim%20Montage%20Object%20Reference))
  ;[0.15 0.15 0.15 0.5] reproduce una animacion setteada desde otro BP
  (|CallParentFunction MontageToPlay)
  (Utilities|FlowControl|Sequence
    (:then_0
      (Input|DisableInput (Game|GetPlayerController 0)) ; desactiva el movimiento
      (Animation|Montage|MontagePlay (Components|SkeletalMesh|GetAnimInstance (Variables|Character|GetMesh)) MontageToPlay 1.0 "MontageLength" 0.0 true)
      (Utilities|FlowControl|Delay 2.0)
      (Input|EnableInput (Game|GetPlayerController 0)) ; Activa el movimiento
    )
    (:then_1
      ;[0.15 0.15 0.15 0.5] Set Rotacion to Interact Target
      (bind _newtrack_0 (Timeline|Timeline PlayFromStart)
        (:Update
          (Transformation|SetActorRotation (Math|Interpolation|RInterpTo (Transformation|GetActorRotation) (Math|Rotator|MakeRotator 0.0 0.0 (.Yaw (Math|Rotator|BreakRotator (Math|Rotator|FindLookatRotation (Transformation|GetActorLocation) (Transformation|GetActorLocation (Variables|Default|GetOverlappingInteractItem)))))) _newtrack_0 2.0)))))))

(event EventTick
  (params (DeltaSeconds :type Float%20%28single-precision%29))
  ;[0.15 0.15 0.15 0.5] Setteamos materiales dinamicos
  (Variables|Default|SetTime DeltaSeconds)
  (bind _outhit (Collision|LineTraceByChannel (Transformation|GetWorldLocation (Variables|Default|GetFollowCamera)) (Transformation|GetWorldLocation (Variables|Default|GetHair)) "TraceTypeQuery1" false 0 "None"))
  (if (.bBlockingHit (Collision|BreakHitResult _outhit))
    (bind _output_get (Variables|Default|SetHit%20Actor (.HitActor (Collision|BreakHitResult _outhit))))
    (if (Actor|ActorHasTag _output_get "Translucent")
      ;;[0.15 0.15 0.15 0.5] si es un arbgol
      (if (Class|GameplayStatics|ObjectIsA _output_get "/Game/Blueprints/Items/BP_Tree.BP_Tree_C")
        (Utilities|FlowControl|Sequence
          (:then_0
            (Utilities|FlowControl|DoOnce false :!label _label
              (:Completed
                (bind _asbp_tree (Utilities|Casting|CastToBP_Tree (Variables|Default|GetHit%20Actor)))
                (Variables|Default|SetAs%20BP%20Tree_0 _asbp_tree))))
          (:then_1
            (if (not (<= (Variables|Default|GetCurrent%20Value) 0.0))
              (bind _output_get_2 (Variables|Default|SetCurrent%20Value (Math|Float|Lerp (Variables|Default|GetCurrent%20Value) (- (Variables|Default|GetCurrent%20Value) 0.3) (* (Variables|Default|GetTime) 9.0))))
              (Rendering|Material|SetScalarParameterValue (Variables|/Game/Blueprints/Items/BP_Tree.BP_Tree_C|GetMaterialInstanceRef (Variables|Default|GetAs%20BP%20Tree_0)) "Show FadeOut Effect" _output_get_2 :!class /Script/Engine.MaterialInstanceDynamic)
              (Rendering|Material|SetScalarParameterValue (Variables|/Game/Blueprints/Items/BP_Tree.BP_Tree_C|GetMaterialInstanceLevaces (Variables|Default|GetAs%20BP%20Tree_0)) "Show FadeOut Effect" _output_get_2 :!class /Script/Engine.MaterialInstanceDynamic))))
        (elif (Class|GameplayStatics|ObjectIsA _output_get "/Game/Blueprints/Items/BP_Rock.BP_Rock_C")
          (Utilities|FlowControl|DoOnce false
            (:Completed
              (bind _asbp_tree_2 (Utilities|Casting|CastToBP_Tree (Variables|Default|GetHit%20Actor)))
              (Variables|Default|SetAs%20BP%20Tree_0 _asbp_tree_2))))))
    (else
      (bind _as_bp_tree_0 (Variables|Default|GetAs%20BP%20Tree_0)
        (:then
          (if (Class|GameplayStatics|ObjectIsA _as_bp_tree_0 "/Game/Blueprints/Items/BP_Tree.BP_Tree_C")
            (if (>= (Variables|Default|GetCurrent%20Value) 1.0)
              (Variables|Default|SetAs%20BP%20Tree_0 0)
              (goto _label Reset)
              (else
                (bind _output_get_3 (Variables|Default|SetCurrent%20Value (Math|Float|Lerp (Variables|Default|GetCurrent%20Value) (+ (Variables|Default|GetCurrent%20Value) 0.5) (* (Variables|Default|GetTime) 1e+01))))
                (Rendering|Material|SetScalarParameterValue (Variables|/Game/Blueprints/Items/BP_Tree.BP_Tree_C|GetMaterialInstanceRef _as_bp_tree_0) "Show FadeOut Effect" _output_get_3 :!class /Script/Engine.MaterialInstanceDynamic)
                (Rendering|Material|SetScalarParameterValue (Variables|/Game/Blueprints/Items/BP_Tree.BP_Tree_C|GetMaterialInstanceLevaces (Variables|Default|GetAs%20BP%20Tree_0)) "Show FadeOut Effect" _output_get_3 :!class /Script/Engine.MaterialInstanceDynamic)))
            (elif (Class|GameplayStatics|ObjectIsA _as_bp_tree_0 "/Game/Blueprints/Items/BP_Rock.BP_Rock_C")
              _)))
        (:else)))))

(event EventSetAmountOfElementstoPlayer
  (params (Rocks :type Integer) (Flowers :type Integer) (Trees :type Integer) (Lights :type Integer))
  ;[0.15 0.15 0.15 0.5] Settea el valor inicial de los objetos en el escenario
  (|CallParentFunction Rocks Flowers Trees Lights)
  (bind _output_get (Variables|Default|SetAmountOfRocks Rocks))
  (Variables|Default|SetCurrentAmountOfRocks _output_get)
  (bind _output_get_2 (Variables|Default|SetAmountOfFlowers Flowers))
  (Variables|Default|SetCurrentAmountOfFlowers _output_get_2)
  (bind _output_get_3 (Variables|Default|SetAmountOfTrees Trees))
  (Variables|Default|SetCurrentAmountOfTrees _output_get_3)
  (bind _output_get_4 (Variables|Default|SetAmountOfLights Lights))
  (Variables|Default|SetCurrentAmountOfLights _output_get_4))

(event EventSetAmountOfElementstoWidget
  (params (Rocks :type Integer) (Flowers :type Integer) (Trees :type Integer) (Lights :type Integer))
  ;[0.15 0.15 0.15 0.5] Setea el texto en el wiget
  (Variables|/Game/UI/Texts/WB_ElementsManager.WB_ElementsManager_C|SetRocks%20amount (Variables|Widgets|GetWB_ElementsAmount) (Utilities|Text|ToText(Integer) Rocks))
  (Variables|/Game/UI/Texts/WB_ElementsManager.WB_ElementsManager_C|SetFlower_Amount (Variables|Widgets|GetWB_ElementsAmount) (Utilities|Text|ToText(Integer) Flowers))
  (Variables|/Game/UI/Texts/WB_ElementsManager.WB_ElementsManager_C|SetTree_Amount (Variables|Widgets|GetWB_ElementsAmount) (Utilities|Text|ToText(Integer) Trees))
  (Variables|/Game/UI/Texts/WB_ElementsManager.WB_ElementsManager_C|SetLight_Amount (Variables|Widgets|GetWB_ElementsAmount) (Utilities|Text|ToText(Integer) Lights)))

(event EventUpdateSpawnerDataBP
  (|CallParentFunction)
  (if (<= (Variables|Default|GetCurrentAmountOfTrees) (/ (Variables|Default|GetAmountOfTrees) 2))
    (Default|CallEDSpawnObjects)))

(fn ConstructionScript)

(fn FActivatePropsLastLevel
  (params (InputPin :type Actor%20Object%20Reference))
  (if (Class|GameplayStatics|ObjectIsA InputPin "/Game/Blueprints/Items/BP_Flower.BP_Flower_C")
    (bind _asbp_flower (Utilities|Casting|CastToBP_Flower InputPin))
    (bind _output_get (Variables|Default|SetAs%20BP%20Flower _asbp_flower))
    (Class|TouchingInterface|WateringPlantBP _output_get)
    (Class|TouchingInterface|TouchingBP _output_get)
    (elif (Class|GameplayStatics|ObjectIsA InputPin "/Game/Blueprints/Items/BP_Tree.BP_Tree_C")
      (bind _asbp_tree (Utilities|Casting|CastToBP_Tree InputPin))
      (bind _output_get_2 (Variables|Default|SetAs%20BP%20Tree _asbp_tree))
      (Class|TouchingInterface|TouchingBP _output_get_2)
      (elif (Class|GameplayStatics|ObjectIsA InputPin "/Game/Blueprints/Items/BP_Rock.BP_Rock_C")
        (bind _asbp_rock (Utilities|Casting|CastToBP_Rock InputPin))
        (bind _output_get_3 (Variables|Default|SetAs%20BP%20Rock _asbp_rock))
        (Class|TouchingInterface|TouchingBP _output_get_3)))))

(fn SetInitialAmounttoWidget
  (Variables|/Game/UI/Texts/WB_ElementsManager.WB_ElementsManager_C|SetRocks%20amount (Variables|Widgets|GetWB_ElementsAmount) (Utilities|Text|ToText(Integer) (Variables|Default|GetAmountOfRocks)))
  (Variables|/Game/UI/Texts/WB_ElementsManager.WB_ElementsManager_C|SetFlower_Amount (Variables|Widgets|GetWB_ElementsAmount) (Utilities|Text|ToText(Integer) (Variables|Default|GetAmountOfFlowers))))

(fn OverlappingIsAFlower
  (bind _overlappinginteractitem (Variables|Default|GetOverlappingInteractItem)
    (:then
      (if (Class|GameplayStatics|ObjectIsA _overlappinginteractitem "/Game/Blueprints/Items/BP_Flower.BP_Flower_C")
        (bind _asbp_flower (Utilities|Casting|CastToBP_Flower _overlappinginteractitem))
        (bind _output_get (Variables|Default|SetAs%20BP%20Flower_0 _asbp_flower))
        (return _output_get)))
    (:else)))