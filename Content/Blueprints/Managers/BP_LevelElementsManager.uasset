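; Level elements manager that counts the collectible or placed element actors in the current level and reports them to BP_WorldPlayer and its amount widget.
; Shortly after BeginPlay it branches on level name, counting actors with GetAllActorsOfClass.
; Setup is cumulative: LvL_One counts rocks, LvL_Two adds flowers and trees, LvL_Three and LvL_Four add candles as lights.
; Later levels also reveal the matching widget icons.
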(event Custom|SetInitial%20Values
  (bind _as_bp_world_player (Variables|Default|GetAs%20BP%20World%20Player))
  ;[0.15 0.15 0.15 0.5] Settea nivel uno
  (Utilities|FlowControl|Delay 0.2)
  (bind _returnvalue (Game|GetCurrentLevelName true))
  (if (Utilities|Enum|Equal(Enum) _returnvalue "LvL_One")
    (bind _outactors (Actor|GetAllActorsOfClass "/Game/Blueprints/Items/BP_Rock.BP_Rock_C"))
    (bind _output_get (Variables|Default|SetRocksAmount _outactors))
    (Class|WorldPlayer|SetAmountOfElementstoPlayer (Variables|Default|GetAs%20BP%20World%20Player) (Utilities|Array|Length _output_get))
    (Class|WorldPlayer|SetAmountOfElementstoWidget (Variables|Default|GetAs%20BP%20World%20Player) (Variables|/Script/MyWorld.WorldPlayer|GetCurrentAmountOfRocks _as_bp_world_player) (Variables|/Script/MyWorld.WorldPlayer|GetCurrentAmountOfFlowers _as_bp_world_player) (Variables|/Script/MyWorld.WorldPlayer|GetCurrentAmountOfTrees _as_bp_world_player) (Variables|/Script/MyWorld.WorldPlayer|GetCurrentAmountOfLights _as_bp_world_player) :!label _label)
    (else
      ;[0.15 0.15 0.15 0.5] Settea nivel dos
      (bind _returnvalue_2 (Game|GetCurrentLevelName true))
      (if (Utilities|Enum|Equal(Enum) _returnvalue_2 "LvL_Two")
        (CallFunction|SetLevel2)
        (else
          ;[0.15 0.15 0.15 0.5] settea nivel 3
          (bind _returnvalue_3 (Game|GetCurrentLevelName true))
          (if (Utilities|Enum|Equal(Enum) _returnvalue_3 "LvL_Three")
            (Utilities|FlowControl|Sequence :!label _label_2
              (:then_0
                (CallFunction|SetLevel2))
              (:then_1
                (bind _outactors_2 (Actor|GetAllActorsOfClass "/Game/Blueprints/Items/BP_Candle.BP_Candle_C"))
                (bind _output_get_2 (Variables|Default|SetCandlesAmount _outactors_2))
                (Class|WorldPlayer|SetAmountOfElementstoPlayer (Variables|Default|GetAs%20BP%20World%20Player) (Utilities|Array|Length _output_get) (Utilities|Array|Length (stale Custom|Set%20Level%202 _output_get_2)) (Utilities|Array|Length (stale Custom|Set%20Level%202 _output_get_3)) (Utilities|Array|Length _output_get_2))
                (goto _label))
              (:then_2
                (Variables|/Game/UI/Texts/WB_ElementsManager.WB_ElementsManager_C|SetCandlesIconVisibility (Variables|/Game/Blueprints/Player/BP_WorldPlayer.BP_WorldPlayer_C|GetWB_ElementsAmount (Variables|Default|GetAs%20BP%20World%20Player)) "Visible")))
            (else
              (bind _returnvalue_4 (Game|GetCurrentLevelName true))
              (if (Utilities|Enum|Equal(Enum) _returnvalue_4 "LvL_Four")
                (goto _label_2)))))))))

(event Custom|Set%20Level%202
  (bind _as_bp_world_player (Variables|Default|GetAs%20BP%20World%20Player))
  (bind _as_bp_world_player_2 (Variables|Default|GetAs%20BP%20World%20Player))
  (bind _wb_elementsamount (Variables|/Game/Blueprints/Player/BP_WorldPlayer.BP_WorldPlayer_C|GetWB_ElementsAmount _as_bp_world_player_2))
  ;[0.15 0.15 0.15 0.5] Settea nivel dos
  (Utilities|FlowControl|Sequence
    (:then_0
      ;[0.15 0.15 0.15 0.5] Settea nivel uno
      (bind _outactors (Actor|GetAllActorsOfClass "/Game/Blueprints/Items/BP_Rock.BP_Rock_C"))
      (bind _output_get (Variables|Default|SetRocksAmount _outactors))
      (Class|WorldPlayer|SetAmountOfElementstoPlayer (Variables|Default|GetAs%20BP%20World%20Player) (Utilities|Array|Length _output_get))
      (Class|WorldPlayer|SetAmountOfElementstoWidget (Variables|Default|GetAs%20BP%20World%20Player) (Variables|/Script/MyWorld.WorldPlayer|GetCurrentAmountOfRocks _as_bp_world_player) (Variables|/Script/MyWorld.WorldPlayer|GetCurrentAmountOfFlowers _as_bp_world_player) (Variables|/Script/MyWorld.WorldPlayer|GetCurrentAmountOfTrees _as_bp_world_player) (Variables|/Script/MyWorld.WorldPlayer|GetCurrentAmountOfLights _as_bp_world_player) :!label _label))
    (:then_1
      (bind _outactors_2 (Actor|GetAllActorsOfClass "/Game/Blueprints/Items/BP_Flower.BP_Flower_C"))
      (bind _output_get_2 (Variables|Default|SetFlowersAmount _outactors_2))
      (Class|WorldPlayer|SetAmountOfElementstoPlayer (Variables|Default|GetAs%20BP%20World%20Player) (Utilities|Array|Length _output_get) (Utilities|Array|Length _output_get_2) (Utilities|Array|Length (stale _output_get_3)) :!label _label_2)
      (goto _label))
    (:then_2
      (bind _outactors_3 (Actor|GetAllActorsOfClass "/Game/Blueprints/Items/BP_Tree.BP_Tree_C"))
      (bind _output_get_3 (Variables|Default|SetTreeAmount _outactors_3))
      (goto _label_2))
    (:then_3
      (Variables|/Game/UI/Texts/WB_ElementsManager.WB_ElementsManager_C|SetFlowerIconVisibility _wb_elementsamount "Visible")
      (Variables|/Game/UI/Texts/WB_ElementsManager.WB_ElementsManager_C|SetTreeIconVisibility _wb_elementsamount "Visible"))))

(event EventBeginPlay
  (bind _asbp_world_player (Utilities|Casting|CastToBP_WorldPlayer (Game|GetPlayerCharacter 0)))
  (Variables|Default|SetAs%20BP%20World%20Player _asbp_world_player)
  (CallFunction|SetInitialValues))

(fn ConstructionScript)